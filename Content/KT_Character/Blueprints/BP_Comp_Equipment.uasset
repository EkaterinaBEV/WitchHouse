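; Character equipment component that equips items into Hand and Neck slots on the owning BP_Character.
; EquipItem clears the slot, then attaches hand items to the Skt_Weapon socket or casts neck items to Item_Amulet.
; Amulets attach to the character mesh and follow its animation through master pose.
; UnequipItem only clears the stored reference, without detaching the item.
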(event EventBeginPlay
  (bind _asbp_character (Utilities|Casting|CastToBP_Character (Components|GetOwner)))
  (Variables|Default|SetCharacter _asbp_character))

(fn EquipItem
  (params (Item :type BP%20Item%20Equippable%20Object%20Reference) (Part :type BPE_PartsToEquip%20Enum :default "NewEnumerator0"))
  (LocalVariables|SetL_Item Item)
  (CallFunction|UnequipItem Part)
  (switch Utilities|FlowControl|Switch|SwitchonBPE_PartsToEquip Part
    (:NewEnumerator0
      (Variables|Default|SetObjectToHand (LocalVariables|GetL_Item))
      (CallFunction|AttachItem true))
    (:NewEnumerator1
      (CallFunction|EquipAmulets (LocalVariables|GetL_Item))))
  (return true))

(fn UnequipItem
  (params (Part :type BPE_PartsToEquip%20Enum :default "NewEnumerator0"))
  (if (.Equipped (CallFunction|PartEquipped Part))
    (switch Utilities|FlowControl|Switch|SwitchonBPE_PartsToEquip Part
      (:NewEnumerator0
        (Variables|Default|SetObjectToHand 0))
      (:NewEnumerator1
        (Variables|Default|SetNeck 0)))
    (return false)
    (else
      (return true))))

(fn PartEquipped
  (params (Part :type BPE_PartsToEquip%20Enum :default "NewEnumerator0"))
  (bind _objecttohand (Variables|Default|GetObjectToHand))
  (bind _neck (Variables|Default|GetNeck))
  (bind _returnvalue (Utilities|Select :Index Part :NewEnumerator0 _objecttohand :NewEnumerator1 _neck))
  (return (Utilities|IsValid _returnvalue) _returnvalue))

(fn AttachItem
  (params (Attach :type Boolean))
  (Utilities|IsValid (Variables|Default|GetObjectToHand)
    (:Is%20Valid
      (if Attach
        (Transformation|AttachComponentToComponent (Variables|Default|GetObjectToHand) (Variables|/Game/KT_Character/Blueprints/BP_Character.BP_Character_C|GetSkeletalMesh (Variables|Default|GetCharacter)) "Skt_Weapon" "SnapToTarget" "KeepRelative" "KeepRelative" true)
        (else
          (Transformation|DetachFromActor (Variables|Default|GetObjectToHand) "KeepRelative" "KeepRelative" "KeepRelative"))))))

(fn EquipAmulets
  (params (Item :type BP%20Storage%20Item%20Object%20Reference))
  (bind _asitem_amulet (Utilities|Casting|CastToItem_Amulet Item))
  (bind _output_get (Variables|Default|SetNeck _asitem_amulet))
  (CallFunction|AttachAmulets _output_get))

(fn AttachAmulets
  (params (Amulet :type Item%20Amulet%20Object%20Reference))
  (Utilities|IsValid Amulet
    (:Is%20Valid
      (Transformation|AttachComponentToComponent Amulet (Variables|/Script/Engine.Character|GetMesh (Variables|Default|GetCharacter)) "None" "SnapToTarget" "SnapToTarget" "SnapToTarget" true)
      (Class|SkinnedMeshComponent|SetMasterPoseComponent (Variables|/Game/KT_Storage/Storage/Items/EquippableItems/Amulets/Item_Amulet.Item_Amulet_C|GetSkeletalAmulet Amulet) (Variables|/Script/Engine.Character|GetMesh (Variables|Default|GetCharacter)) false)
      (Development|PrintString "Attached!" true true "(R=0.000000,G=0.660000,B=1.000000,A=1.000000)" 5.0))))