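; BP_Comp_Papers is a storage component that holds paper items in a one-dimensional row of slots indexed by Y.
; AddPaper scans upward from the paper's own position for a free slot, then stores it, informs the paper and signals a storage update.
; Slot checks test bounds and the stored papers' positions.
; A separate capacity check compares total stored size plus class-default size times quantity against StorageSize.
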(event EventBeginPlay)

(fn AddPaper
  (params (Item :type Item%20Paper%20Object%20Reference))
  (bind _output_get (LocalVariables|SetPaperToAdd Item))
  (bind (_canadd _y) (CallFunction|IfPaperCanbeAdded _output_get))
  (if _canadd
    (Utilities|Array|Add (Variables|Default|GetItems) (LocalVariables|GetPaperToAdd))
    (Default|PaperAddedtoStorage (LocalVariables|GetPaperToAdd) self _y)
    (Default|CallPaperStorageUpdated)
    (return true)
    (else
      (return false))))

(fn IfPaperCanbeCreated
  (params (Item :type BP%20Storage%20Item%20Class%20Reference) (Quantity :type Integer))
  (if (> (+ (Variables|Default|GetStorageItemsTotalSize) (* (.Size (Utilities|GetClassDefaults Item)) Quantity)) (Variables|Default|GetStorageSize))
    (return false)
    (else
      (return true))))

(fn IfPaperCanbeAdded
  (params (Item :type Item%20Paper%20Object%20Reference))
  (bind (_occupied _y) (CallFunction|CheckFreeSlotforPaper Item (Default|LocatePaper Item)))
  (if (not _occupied)
    (return true _y)
    (else
      (return false 0))))

(fn ChangeTotalSize
  (params (Value :type Integer))
  (Variables|Default|SetStorageItemsTotalSize (+ Value (Variables|Default|GetStorageItemsTotalSize))))

(fn GetPapers
  (return (Variables|Default|GetItems)))

(fn FindPaperinStoragebyClass
  (params (Class :type Item%20Paper%20Class%20Reference))
  (bind _array_element (Utilities|Array|ForEachLoopwithBreak (Variables|Default|GetItems) :!label _label)
    (:LoopBody
      (if (== (Utilities|GetClass _array_element) Class)
        (LocalVariables|SetL_Item _array_element)
        (LocalVariables|SetL_ItemFound true)
        (goto _label Break)))
    (:Completed
      (return (LocalVariables|GetL_Item) (LocalVariables|GetL_ItemFound)))))

(fn CheckSlot
  (params (Y :type Integer) (CheckExactSlotPos :type Boolean))
  (LocalVariables|SetL_Y Y)
  (Utilities|FlowControl|Sequence
    (:then_0
      ;[1 1 1] Check for inventory borders
      (if (or (>= (LocalVariables|GetL_Y) (Variables|Default|GetStorageSize)) (< (LocalVariables|GetL_Y) 0))
        (return 0 false)))
    (:then_1
      (bind _array_element (Utilities|Array|ForEachLoopwithBreak (Variables|Default|GetItems) :!label _label)
        (:LoopBody
          (if (select CheckExactSlotPos (|CheckExactLocation _array_element) (Default|CheckifPaperIsinSlot _array_element (LocalVariables|GetL_Y)))
            (LocalVariables|SetL_Item _array_element)
            (goto _label Break)))))
    (:then_2
      (return (LocalVariables|GetL_Item) (not (Utilities|IsValid (LocalVariables|GetL_Item)))))))

(fn CheckFreeSlotforPaper
  (params (Item :type Item%20Paper%20Object%20Reference) (New%20Y :type Integer))
  (LocalVariables|SetL_Item Item)
  (bind _index (Utilities|FlowControl|ForLoopwithBreak New%20Y (- (Variables|Default|GetStorageSize) 1))
    (:LoopBody
      (bind _output_get (LocalVariables|SetL_Y _index))
      (bind _free (CallFunction|CheckSlot _output_get false))
      (if _free
        ;[1 1 1] Проверяет на размер предмета (у меня некоторые предметы весят 0)
        (bind _slotsarefree (CallFunction|CheckSlotsforPaper (LocalVariables|GetL_Item) (LocalVariables|GetL_Y)))
        (if _slotsarefree
          (return false (LocalVariables|GetL_Y)))))
    (:Completed
      (return true 0))))

(fn CheckSlotsforPaper
  (params (Item :type Item%20Paper%20Object%20Reference) (Y :type Integer))
  (LocalVariables|SetL_Item Item)
  (bind _output_get (LocalVariables|SetL_Y Y))
  (bind _free (CallFunction|CheckSlot (Default|LocatePaper (LocalVariables|GetL_Item)) false))
  (if (or _free (!= _output_get (Default|LocatePaper (LocalVariables|GetL_Item))))
    (return true)
    (else
      (return false))))