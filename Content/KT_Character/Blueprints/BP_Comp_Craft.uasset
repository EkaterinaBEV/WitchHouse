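; Crafting component that turns item actors into a recipe's output item, using food, weapon or amulet recipe DataTables chosen by RecipesDataType.
; FindRecipeByItems returns the first recipe whose required classes are all present, ignoring quantities.
; FindItemsByRecepie picks items with sufficient quantity for a given recipe.
; Craft removes one matching item actor per ingredient, then spawns the output at a far-off location with physics frozen and calls Crafted on it.
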(event EventBeginPlay)

(event EventTick
  (params (DeltaSeconds :type Float%20%28single-precision%29)))

(fn Craft
  (params (Recipe :type ST%20Craft%20Recipe%20Structure) (Items :type Array%20of%20BP%20Storage%20Item%20Object%20References))
  (bind (_outitem _neededitems) (Utilities|Struct|BreakST_CraftRecipe Recipe))
  (bind (_item _quantity) (Utilities|Struct|BreakST_InitialItemsInfo _outitem))
  (Utilities|FlowControl|Sequence
    (:then_0
      (CallFunction|RemoveItemsforCraft Items _neededitems))
    (:then_1
      (bind _returnvalue (Game|SpawnActorfromClass _item (Math|Transform|MakeTransform "999999.000000,999999.000000,999999.000000") "AlwaysSpawn" 0 _quantity 0))
      (Default|FreezePhyzComponents _returnvalue true)
      (Rendering|SetActorHiddenInGame _returnvalue false)
      (Default|Crafted _returnvalue)
      (return _returnvalue))))

(fn FindRecipebyItems
  (params (Items :type Array%20of%20BP%20Storage%20Item%20Object%20References))
  ;[1 1 1] Сперва набираем предметы
  (LocalVariables|SetL_Items Items)
  (bind _rows (CallFunction|GetCraftDataRowNames))
  (bind _array_element (Utilities|Array|ForEachLoopwithBreak _rows :!label _label)
    (:LoopBody
      (bind _row (CallFunction|GetCraftDataRow _array_element))
      (bind _output_get (LocalVariables|SetL_Recipe _row))
      (LocalVariables|SetL_ItemsForRecipeWereNotFound false)
      (bind _array_element_2 (Utilities|Array|ForEachLoopwithBreak (Utilities|Struct|BreakST_CraftRecipe _output_get) :!label _label_2)
        (:LoopBody
          (LocalVariables|SetInitialItemsInfo _array_element_2)
          (LocalVariables|SetL_NeededItemsFound false)
          (bind _array_element_3 (Utilities|Array|ForEachLoopwithBreak (LocalVariables|GetL_Items) :!label _label_3)
            (:LoopBody
              (if (== (.Item (Utilities|Struct|BreakST_InitialItemsInfo (LocalVariables|GetInitialItemsInfo))) (Utilities|GetClass _array_element_3))
                (LocalVariables|SetL_NeededItemsFound true)
                (goto _label_3 Break)))
            (:Completed
              (if (not (LocalVariables|GetL_NeededItemsFound))
                (LocalVariables|SetL_ItemsForRecipeWereNotFound true)
                (goto _label_2 Break)))))
        (:Completed
          (if (not (LocalVariables|GetL_ItemsForRecipeWereNotFound))
            (LocalVariables|SetL_RecipeWasFound true)
            (goto _label Break)))))
    (:Completed
      (return (LocalVariables|GetL_Recipe) (LocalVariables|GetL_RecipeWasFound)))))

(fn FindItemsbyRecepie
  (params (Recipe :type ST%20Craft%20Recipe%20Structure) (InitItems :type Array%20of%20BP%20Storage%20Item%20Object%20References))
  ;[1 1 1] Сперва получаем рецепт
  (LocalVariables|SetL_InitItems InitItems)
  (bind _array_element (Utilities|Array|ForEachLoopwithBreak (Utilities|Struct|BreakST_CraftRecipe Recipe))
    (:LoopBody
      (bind _array_element_2 (Utilities|Array|ForEachLoopwithBreak (LocalVariables|GetL_InitItems) :!label _label)
        (:LoopBody
          (if (== (Utilities|GetClass _array_element_2) (.Item (Utilities|Struct|BreakST_InitialItemsInfo _array_element)))
            (bind _output_get (LocalVariables|SetL_TempItem _array_element_2))
            (Utilities|IsValid _output_get
              (:Is%20Valid
                (if (< (Variables|/Game/KT_Storage/Storage/Items/BP_StorageItem.BP_StorageItem_C|GetQuantity _output_get) (.Quantity (Utilities|Struct|BreakST_InitialItemsInfo _array_element)))
                  (LocalVariables|SetL_Found false)
                  (else
                    (Utilities|Array|Add (LocalVariables|GetL_Items) (LocalVariables|GetL_TempItem))
                    (LocalVariables|SetL_Found true)
                    (goto _label Break)))))))
        (:Completed
          (if (not (LocalVariables|GetL_Found))
            (return false (Utilities|Array|MakeArray))))))
    (:Completed
      (return (LocalVariables|GetL_Found) (LocalVariables|GetL_Items)))))

(fn RemoveItemsforCraft
  (params (NeededItems :type Array%20of%20BP%20Storage%20Item%20Object%20References) (Info :type Array%20of%20ST%20Initial%20Items%20Info%20Structures))
  (LocalVariables|SetL_NeededItems NeededItems)
  (for _array_element Info
    (bind (_array_element_2 _array_index) (Utilities|Array|ForEachLoopwithBreak (LocalVariables|GetL_NeededItems) :!label _label)
      (:LoopBody
        (if (== (Utilities|GetClass _array_element_2) (.Item (Utilities|Struct|BreakST_InitialItemsInfo _array_element)))
          (Default|RemoveItem _array_element_2)
          (Utilities|Array|RemoveIndex (LocalVariables|GetL_NeededItems) _array_index)
          (goto _label Break))))))

(fn GetCraftDataRow
  (params (RowName :type Name))
  (LocalVariables|SetL_RowName RowName)
  (Utilities|FlowControl|Sequence
    (:then_0
      (switch Utilities|FlowControl|Switch|SwitchonE_RecipeDataTypes (Variables|Default|GetRecipesDataType)
        (:NewEnumerator0
          (bind _returnvalue (Utilities|GetDataTableRow "/Game/KT_Storage/Recipes/DT_FoodRecipes.DT_FoodRecipes" (LocalVariables|GetL_RowName))
            (:then
              (LocalVariables|SetL_OutRow _returnvalue))))
        (:NewEnumerator1
          (bind _returnvalue_2 (Utilities|GetDataTableRow "/Game/KT_Storage/Recipes/DT_WeaponRecipes.DT_WeaponRecipes" (LocalVariables|GetL_RowName))
            (:then
              (LocalVariables|SetL_OutRow _returnvalue_2))))
        (:NewEnumerator2
          (bind _returnvalue_3 (Utilities|GetDataTableRow "/Game/KT_Storage/Recipes/DT_AmuletRecipes.DT_AmuletRecipes" (LocalVariables|GetL_RowName))
            (:then
              (LocalVariables|SetL_OutRow _returnvalue_3))))))
    (:then_1
      (return (LocalVariables|GetL_OutRow)))))

(fn GetCraftDataRowNames
  (Utilities|FlowControl|Sequence
    (:then_0
      (switch Utilities|FlowControl|Switch|SwitchonE_RecipeDataTypes (Variables|Default|GetRecipesDataType)
        (:NewEnumerator0
          (bind _outrownames (DataTable|GetDataTableRowNames "/Game/KT_Storage/Recipes/DT_FoodRecipes.DT_FoodRecipes"))
          (LocalVariables|SetL_Rows _outrownames))
        (:NewEnumerator1
          (bind _outrownames_2 (DataTable|GetDataTableRowNames "/Game/KT_Storage/Recipes/DT_WeaponRecipes.DT_WeaponRecipes"))
          (LocalVariables|SetL_Rows _outrownames_2))
        (:NewEnumerator2
          (bind _outrownames_3 (DataTable|GetDataTableRowNames "/Game/KT_Storage/Recipes/DT_AmuletRecipes.DT_AmuletRecipes"))
          (LocalVariables|SetL_Rows _outrownames_3))))
    (:then_1
      (return (LocalVariables|GetL_Rows)))))