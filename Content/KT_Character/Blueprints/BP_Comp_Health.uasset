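; Health component for a character that tracks current health and signals when it runs out.
; ChangeHealth adds a signed value without clamping, and on reaching zero sets NoHealth and fires HealthEnded.
; While NoHealth is false, Tick prints health for debugging and runs Regeneration after a delay whenever health differs from maximum.
; Regeneration, noted as not working, applies delta-scaled healing through ChangeHealth when manual or automatic regen is active.
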(event EventTick
  (params (DeltaSeconds :type Float%20%28single-precision%29))
  (if (not (Variables|Default|GetNoHealth))
    (Utilities|FlowControl|Sequence
      (:then_0
        (if (!= (Variables|Default|GetCurrentHealth) (Variables|Default|GetMaxHealth))
          (Utilities|FlowControl|Delay 2.0)
          (CallFunction|Regeneration)))
      (:then_1
        (CallFunction|ShowHealth)))))

(fn ChangeHealth
  (params (Value :type Float%20%28single-precision%29))
  (bind _output_get (Variables|Default|SetCurrentHealth (+ Value (Variables|Default|GetCurrentHealth))))
  (if (and (<= _output_get 0.0) (not (Variables|Default|GetNoHealth)))
    (Variables|Default|SetNoHealth true)
    (Default|CallHealthEnded)
    (else
      (Variables|Default|SetNoHealth false))))

(fn ShowHealth
  (Development|PrintString (Utilities|String|Append "Health: " (Utilities|String|ToString(Float) (Variables|Default|GetCurrentHealth))) true true "(R=0.000000,G=0.660000,B=1.000000,A=1.000000)" 0.0))

(fn Regeneration
  ;[1 1 1] Not working for me
  (Utilities|FlowControl|Sequence
    (:then_0
      (if (Variables|Default|GetAllowAutoRegen)
        (if (< (Variables|Default|GetCurrentHealth) (Variables|Default|GetMaxHealth))
          (Variables|Default|SetAutoRegen true)
          (elif (>= (Variables|Default|GetCurrentHealth) (Variables|Default|GetMaxHealth))
            (Variables|Default|SetAutoRegen false)))))
    (:then_1
      (if (or (Variables|Default|GetRegenerate) (Variables|Default|GetAutoRegen))
        (CallFunction|ChangeHealth (* (Variables|Default|GetRegenerationSpeed) (Utilities|Time|GetWorldDeltaSeconds)))))))