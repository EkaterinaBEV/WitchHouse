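; Choppable tree that loses health only to axe damage, falls when depleted, and can then be harvested.
; AnyDamage feeds HittingTree; every non-felling hit, from any source, spawns a berry food actor around Sphere1.
; Felling sets Fallen and fires the TreeIsFalling dispatcher, self-bound on BeginPlay to a timeline that pitches the actor toward 90 degrees.
; Interacting with a fallen tree adds firewood to the character's storage component and destroys the tree.
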(event Custom|FallingTreeAnimation
  (params (Tree :type BP%20Tree%20Object%20Reference) (Instigator :type Pawn%20Object%20Reference))
  (bind _returnvalue (Transformation|GetActorRotation))
  ;[1 1 1] Falling tree animation
  (bind _newtrack_0 (Timeline|FallingTreeAnim Play)
    (:Update
      (Transformation|SetActorRotation (Math|Rotator|MakeRotator (.roll _returnvalue) (Math|Float|Lerp (.pitch _returnvalue) 9e+01 _newtrack_0) (.yaw _returnvalue))))))

(event Game|Damage|EventAnyDamage
  (params (Damage :type Float%20%28single-precision%29) (DamageType :type Damage%20Type%20Object%20Reference) (InstigatedBy :type Controller%20Object%20Reference) (DamageCauser :type Actor%20Object%20Reference))
  ;[1 1 1] Tree was hit
  (CallFunction|HittingTree Damage InstigatedBy DamageCauser))

(event EventBeginPlay
  ;[1 1 1] Falling tree animation
  (EventDispatchers|BindEventtoTreeIsFalling (delegate Custom|FallingTreeAnimation)))

(fn ConstructionScript)

(fn HittingTree
  (params (Damage :type Float%20%28single-precision%29) (Instigator :type Controller%20Object%20Reference) (DamageCauser :type Object%20Object%20Reference))
  (if (== (Utilities|GetClass DamageCauser) "/Game/KT_Storage/Storage/Items/Weapon/Melee/BP_Melee_Axe.BP_Melee_Axe_C")
    (bind _output_get (Variables|Default|SetTreeHealth (- (Variables|Default|GetTreeHealth) Damage)))
    (if (and (<= _output_get 0.0) (== (Utilities|GetClass DamageCauser) "/Game/KT_Storage/Storage/Items/Weapon/Melee/BP_Melee_Axe.BP_Melee_Axe_C"))
      (Variables|Default|SetFallen true)
      (Default|CallTreeIsFalling self (Pawn|GetControlledPawn Instigator))
      (Development|PrintString "Savage!")
      (return true true)
      (else
        (CallFunction|SpawnApples)
        (return false true)))
    (else
      (CallFunction|SpawnApples)
      (return false false))))

(fn SpawnApples
  (bind _sphere1 (Variables|Default|GetSphere1))
  (Game|SpawnActorfromClass "/Game/KT_Storage/Storage/Items/Food/BP_Food_Berry.BP_Food_Berry_C" (Math|Transform|MakeTransform (+ (Transformation|GetWorldLocation _sphere1) (* (Math|Random|RandomUnitVector) (Math|Random|RandomFloatinRange (Variables|/Script/Engine.SphereComponent|GetSphereRadius _sphere1) 0.0))) "0, 0, 0" "1,1,1") "AlwaysSpawn" 0 1 0))

(fn Interact
  (params (Character :type BP%20Character%20Object%20Reference))
  (if (Variables|Default|GetFallen)
    (Default|CreateItems (Variables|/Game/KT_Character/Blueprints/BP_Character.BP_Character_C|GetBP_Comp_Storage Character) (Utilities|Array|MakeArray (Utilities|Struct|MakeST_InitialItemsInfo "/Game/KT_Storage/Storage/Items/StorageItems/BP_Item_FireWood.BP_Item_FireWood_C" 1 0 "None")))
    (Actor|DestroyActor)
    (return true "")
    (else
      (return false ""))))