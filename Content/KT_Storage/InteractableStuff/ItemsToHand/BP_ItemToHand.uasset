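; BP_ItemToHand is an interactable item actor that a character equips to a body part and can later drop.
; Interact equips it through the character's BPCompEquipment, records the wearer and disables collision on success.
; UnequipItem calls DroppedToWorld at a point ahead of player 0, regardless of wearer.
; If that succeeds, it clears equip state, detaches, hides the actor, restores collision and returns false.
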(fn ConstructionScript)

(fn Interact
  (params (Character :type BP%20Character%20Object%20Reference))
  (bind _equipped (Default|EquipItem (Variables|/Game/KT_Character/Blueprints/BP_Character.BP_Character_C|GetBP_Comp_Equipment Character) self (Variables|Default|GetEquipPart)))
  (if _equipped
    (Variables|Default|SetEquipToCharacter Character)
    (Variables|Default|SetEquipped true)
    (Collision|SetActorEnableCollision self false)
    (return true "")
    (else
      (return false ""))))

(fn UnequipItem
  (bind _returnvalue (Game|GetPlayerCharacter 0))
  (bind _dropped (CallFunction|DroppedtoWorld (+ (Transformation|GetActorLocation _returnvalue) (* (Transformation|GetActorForwardVector _returnvalue) (Variables|Default|GetDropDistance)))))
  (if _dropped
    (Variables|Default|SetEquipToCharacter 0)
    (Variables|Default|SetEquipped false)
    (Transformation|DetachFromActor "KeepRelative" "KeepRelative" "KeepRelative")
    (Rendering|SetActorHiddenInGame true)
    (Collision|SetActorEnableCollision self true)
    (return false)
    (else
      (return true))))