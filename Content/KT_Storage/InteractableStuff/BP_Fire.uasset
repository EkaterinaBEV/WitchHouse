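; BP_Fire is an interactable fire that damages actors standing in it and doubles as a crafting station.
; Capsule overlaps maintain a list of affected actors, running a looping timer that applies damage to each until the list empties.
; Interact opens the player controller's craft widget, initialized with the fire's storage and craft components, and fails when the character lacks a KT_PlayerController.
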(event OnComponentBeginOverlap(Capsule)
  (params (OverlappedComponent :type Primitive%20Component%20Object%20Reference) (OtherActor :type Actor%20Object%20Reference) (OtherComp :type Primitive%20Component%20Object%20Reference) (OtherBodyIndex :type Integer) (bFromSweep :type Boolean) (SweepResult :type Hit%20Result%20Structure%20%28by%20ref%29))
  ;[1 1 1] Checking for other actors
  (Utilities|Array|AddUnique (Variables|Default|GetActorsGettingDamage) OtherActor)
  (if (not (Utilities|Time|IsValidTimerHandle (Variables|Default|GetDamageTimer)))
    (bind _returnvalue (Utilities|Time|SetTimerbyFunctionName 0 "DamageActors" (Variables|Default|GetDamageDelay) true))
    (Variables|Default|SetDamageTimer _returnvalue)))

(event OnComponentEndOverlap(Capsule)
  (params (OverlappedComponent :type Primitive%20Component%20Object%20Reference) (OtherActor :type Actor%20Object%20Reference) (OtherComp :type Primitive%20Component%20Object%20Reference) (OtherBodyIndex :type Integer))
  (bind _actorsgettingdamage (Variables|Default|GetActorsGettingDamage))
  ;[1 1 1] Deleting all actors getting damage
  (Utilities|Array|RemoveItem _actorsgettingdamage OtherActor)
  (if (== (Utilities|Array|Length _actorsgettingdamage) 0)
    (Utilities|Time|ClearandInvalidateTimerbyHandle (Variables|Default|GetDamageTimer))
    (Variables|Default|SetDamageTimer "")))

(fn ConstructionScript)

(fn DamageActors
  (bind _output_get (LocalVariables|SetL_Actors (Variables|Default|GetActorsGettingDamage)))
  (for _array_element _output_get
    (Game|Damage|ApplyDamage _array_element (Variables|Default|GetDamage) 0 self)))

(fn Interact
  (params (Character :type BP%20Character%20Object%20Reference))
  (bind _askt_player_controller (Utilities|Casting|CastToKT_PlayerController (Pawn|GetController Character))
    (:then
      (bind _craftwidget (Default|CraftWidget _askt_player_controller true))
      (Default|InitCraftGrid _craftwidget (Variables|Default|GetBP_StorageComponent) (Variables|Default|GetBP_Comp_Craft))
      (return true ""))
    (:CastFailed
      (return false "Are you even Alive?"))))