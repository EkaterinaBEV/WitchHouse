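; Equippable item Blueprint in the storage item system, adding equip and unequip behavior to its parent item.
; Equipping stores the character, registers with its BPCompEquipment at the item's Hand slot, then shows the actor with collision off.
; Unequipping clears that state, detaches, and parks the hidden actor at a far-off location with collision back on.
; Dropping to the world first unequips through the component, then runs the parent drop logic.
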(event EventBeginPlay
  (|CallParentFunction) ; This node is disabled and will not be called.\nDrag off pins to build functionality.
)

(event Collision|EventActorBeginOverlap
  (params (OtherActor :type Actor%20Object%20Reference))
  (|CallParentFunction OtherActor) ; This node is disabled and will not be called.\nDrag off pins to build functionality.
)

(event EventTick
  (params (DeltaSeconds :type Float%20%28single-precision%29))
  (|CallParentFunction DeltaSeconds) ; This node is disabled and will not be called.\nDrag off pins to build functionality.
)

(fn ConstructionScript
  (|CallParentFunction))

(fn EquipItem
  (params (EquipToCharacter :type BP%20Character%20Object%20Reference))
  (Variables|Default|SetEquipToCharacter EquipToCharacter)
  (Variables|Default|SetEquipped true)
  (bind _equipped (Default|EquipItem (Variables|/Game/KT_Character/Blueprints/BP_Character.BP_Character_C|GetBP_Comp_Equipment (Variables|Default|GetEquipToCharacter)) self (Variables|Default|GetHand)))
  (Rendering|SetActorHiddenInGame false)
  (Collision|SetActorEnableCollision self false)
  (return _equipped))

(fn UnequipItem
  (Variables|Default|SetEquipToCharacter 0)
  (bind _output_get (Variables|Default|SetEquipped false))
  (Transformation|DetachFromActor "KeepRelative" "KeepRelative" "KeepRelative")
  (Transformation|SetActorLocation "9999.000000,9999.000000,9999.000000" false true)
  (Rendering|SetActorHiddenInGame true)
  (Collision|SetActorEnableCollision self true)
  (return _output_get))

(fn IsItemEquipped
  (return (Variables|Default|GetEquipped) (Variables|Default|GetHand)))

(fn DroppedtoWorld
  (params (Location :type Vector :default "0, 0, 0"))
  (if (Variables|Default|GetEquipped)
    (Default|UnequipItem (Variables|/Game/KT_Character/Blueprints/BP_Character.BP_Character_C|GetBP_Comp_Equipment (Variables|Default|GetEquipToCharacter)) (Variables|Default|GetHand)))
  (bind _dropped (|CallParentFunction Location))
  (return _dropped))