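; BP_Key is an item Blueprint for the storage system whose use action calls Death on the character holding it.
; UseItem checks IsInStorage, casts the storage's owner to BP_Character and returns true after calling Death, or false if either check fails.
; The event graph holds only disabled default events, and the construction script only calls its parent.
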(event EventBeginPlay
  (|CallParentFunction) ; This node is disabled and will not be called.\nDrag off pins to build functionality.
)

(event Collision|EventActorBeginOverlap
  (params (OtherActor :type Actor%20Object%20Reference))
  (|CallParentFunction OtherActor) ; This node is disabled and will not be called.\nDrag off pins to build functionality.
)

(event EventTick
  (params (DeltaSeconds :type Float%20%28single-precision%29))
  (|CallParentFunction DeltaSeconds) ; This node is disabled and will not be called.\nDrag off pins to build functionality.
)

(fn ConstructionScript
  (|CallParentFunction))

(fn UseItem
  (bind (_instorage _storage) (CallFunction|IsinStorage))
  (if _instorage
    (bind _asbp_character (Utilities|Casting|CastToBP_Character (Components|GetOwner _storage))
      (:then
        (Default|Death _asbp_character)
        (return true))
      (:CastFailed
        (return false)))
    (else
      (return false))))