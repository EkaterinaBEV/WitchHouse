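; Melee weapon Blueprint that gates the parent UseWeapon behind an always-true CanUse and provides hit-detection helpers, none called here.
; Hits start at the wielder's location, aimed along their forward vector tilted by controller pitch.
; TraceHit fans line traces and damages each actor once, while SphereTraceHit damages a single hit, both with debug drawing.
; ConeOverlapHit, marked as needing correction, damages overlaps of a temporary scaled mesh component.
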(event EventBeginPlay
  (|CallParentFunction) ; This node is disabled and will not be called.\nDrag off pins to build functionality.
)

(event Collision|EventActorBeginOverlap
  (params (OtherActor :type Actor%20Object%20Reference))
  (|CallParentFunction OtherActor) ; This node is disabled and will not be called.\nDrag off pins to build functionality.
)

(event EventTick
  (params (DeltaSeconds :type Float%20%28single-precision%29))
  (|CallParentFunction DeltaSeconds) ; This node is disabled and will not be called.\nDrag off pins to build functionality.
)

(fn ConstructionScript
  (|CallParentFunction))

(fn ConeOverlapHit
  (params (Radius :type Float%20%28single-precision%29) (Angle :type Float%20%28single-precision%29) (Height :type Float%20%28single-precision%29))
  ;[1 1 1] Needs correction
  (bind _returnvalue (AddComponent|AddStaticMeshComponent true))
  (bind _output_get (LocalVariables|SetL_Collision _returnvalue))
  (Transformation|SetWorldTransform _output_get (Math|Transform|MakeTransform (Transformation|GetActorLocation (Variables|Default|GetEquipToCharacter)) (Math|Conversions|RotationFromXVector (CallFunction|HitDirection)) (Math|Vector|MakeVector Radius (* Radius Angle) Height)) false false)
  (bind _output_get_2 (LocalVariables|SetL_ActorsInCollision (Collision|GetOverlappingActors (LocalVariables|GetL_Collision) "/Script/Engine.Actor" :!class /Script/Engine.PrimitiveComponent)))
  (for _array_element _output_get_2
    (Game|Damage|ApplyDamage _array_element (Variables|Default|GetDamage) (Pawn|GetController (Game|GetInstigator)) self "/Script/Engine.DamageType")
    (Development|PrintString (Utilities|GetDisplayName _array_element)))
  (Components|DestroyComponent (LocalVariables|GetL_Collision)))

(fn TraceHit
  (params (Angle :type Float%20%28single-precision%29) (Radius :type Float%20%28single-precision%29) (TraceQuantity :type Integer))
  (bind _vector (CallFunction|HitInitialLocation))
  (bind _l_actor (LocalVariables|GetL_Actor))
  (for _index (range 0 (- TraceQuantity 1))
    (bind (_outhit _returnvalue) (Collision|LineTraceByChannel _vector (+ _vector (Math|Vector|RotateVectorAroundAxis (* (Math|Vector|RotateVector (Transformation|GetActorForwardVector (Variables|Default|GetEquipToCharacter)) (Math|Rotator|MakeRotator 0.0 0.0 (+ (* _index (/ Angle (Math|Conversions|ToFloat(Integer) TraceQuantity))) (* (/ Angle 2.0) -1.0)))) Radius) (* (.pitch (Transformation|GetActorRotation (Pawn|GetController (Variables|Default|GetEquipToCharacter)))) -1.0) (Transformation|GetActorRightVector (Variables|Default|GetEquipToCharacter)))) "TraceTypeQuery1" false 0 "ForDuration"))
    (if _returnvalue
      (if (not (>= (Utilities|Array|FindItem _l_actor (.HitActor (Collision|BreakHitResult _outhit))) 0))
        (Utilities|Array|Add _l_actor (.HitActor (Collision|BreakHitResult _outhit)))
        (Utilities|Array|Add (LocalVariables|GetL_Hit) _outhit))))
  (for _array_element (LocalVariables|GetL_Hit)
    (CallFunction|DealDamage (Variables|Default|GetDamage) _array_element self)))

(fn HitDirection
  (bind _equiptocharacter (Variables|Default|GetEquipToCharacter))
  (return (Math|Vector|RotateVectorAroundAxis (Transformation|GetActorForwardVector _equiptocharacter) (* (.pitch (Transformation|GetActorRotation (Pawn|GetController _equiptocharacter))) -1.0) (Transformation|GetActorRightVector _equiptocharacter))))

(fn HitInitialLocation
  (return (Transformation|GetActorLocation (Variables|Default|GetEquipToCharacter))))

(fn SphereTraceHit
  (params (Radius :type Float%20%28single-precision%29) (SphereRadius :type Float%20%28single-precision%29))
  (bind _vector (CallFunction|HitInitialLocation))
  (bind (_outhit _returnvalue) (Collision|SphereTraceForObjects _vector (+ _vector (* (CallFunction|HitDirection) Radius)) SphereRadius (Utilities|Array|MakeArray "ObjectTypeQuery3" "ObjectTypeQuery1" "ObjectTypeQuery2" "ObjectTypeQuery5" "ObjectTypeQuery4" "ObjectTypeQuery6") false (Utilities|Array|MakeArray (Variables|Default|GetEquipToCharacter)) "ForDuration"))
  (if _returnvalue
    (CallFunction|DealDamage (Variables|Default|GetDamage) _outhit self)))

(fn UseWeapon
  (if (CallFunction|CanUse)
    (bind (_used _weapon) (|CallParentFunction))
    (return _used _weapon)
    (else
      (return false self))))

(fn CanUse
  (return true))