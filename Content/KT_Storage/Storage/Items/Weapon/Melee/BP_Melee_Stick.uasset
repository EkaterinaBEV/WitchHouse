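; BP_Melee_Stick is a stick melee weapon Blueprint that performs a short-range hit check when used.
; Its UseWeapon override calls the parent first and, only if that reports a successful use, runs SphereTraceHit with stick-specific reach and sphere size.
; It passes the parent's weapon reference and used result back to the caller, and otherwise adds no event or construction logic of its own.
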(event EventBeginPlay
  (|CallParentFunction) ; This node is disabled and will not be called.\nDrag off pins to build functionality.
)

(event Collision|EventActorBeginOverlap
  (params (OtherActor :type Actor%20Object%20Reference))
  (|CallParentFunction OtherActor) ; This node is disabled and will not be called.\nDrag off pins to build functionality.
)

(event EventTick
  (params (DeltaSeconds :type Float%20%28single-precision%29))
  (|CallParentFunction DeltaSeconds) ; This node is disabled and will not be called.\nDrag off pins to build functionality.
)

(fn ConstructionScript
  (|CallParentFunction))

(fn UseWeapon
  (bind (_used _weapon) (|CallParentFunction))
  (if _used
    (CallFunction|SphereTraceHit 1e+02 3e+01)
    (return true _weapon)
    (else
      (return false _weapon))))