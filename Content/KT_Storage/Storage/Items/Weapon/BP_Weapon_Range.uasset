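; Ranged weapon item that spends ammo from its storage on use and provides hitscan and projectile firing helpers.
; UseWeapon finds and caches an ammo item by class, checks CanShoot (always true here), removes ammo, then runs the parent use logic.
; LineTraceShot deals damage along a trace and ProjectileShot spawns a damage-carrying projectile.
; Both aim from the Muzzle socket toward the point found by a screen-center trace.
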(event EventBeginPlay
  (|CallParentFunction) ; This node is disabled and will not be called.\nDrag off pins to build functionality.
)

(event Collision|EventActorBeginOverlap
  (params (OtherActor :type Actor%20Object%20Reference))
  (|CallParentFunction OtherActor) ; This node is disabled and will not be called.\nDrag off pins to build functionality.
)

(event EventTick
  (params (DeltaSeconds :type Float%20%28single-precision%29))
  (|CallParentFunction DeltaSeconds) ; This node is disabled and will not be called.\nDrag off pins to build functionality.
)

(fn ConstructionScript
  (|CallParentFunction))

(fn LineTraceShot
  (bind (_location _direction) (CallFunction|GetShotStartLocation "RTS_World"))
  (bind _outhit (Collision|LineTraceByChannel _location (+ _location (* _direction (Variables|Default|GetFireRange))) "TraceTypeQuery1" false (Utilities|Array|MakeArray (Game|GetInstigator)) "ForDuration"))
  (CallFunction|DealDamage (Variables|Default|GetDamage) _outhit self))

(fn ProjectileShot
  (bind (_location _direction) (CallFunction|GetShotStartLocation "RTS_World"))
  (bind _returnvalue (Game|SpawnActorfromClass (Variables|Default|GetProjectile) (Math|Transform|MakeTransform (+ _location (* _direction 2e+01)) (Math|Conversions|RotationFromXVector _direction)) "AlwaysSpawn" self (Variables|Default|GetDamage) (Variables|Default|GetEquipToCharacter)))
  (return _returnvalue))

(fn GetShotStartLocation
  (params (TransformSpace :type ERelativeTransformSpace%20Enum :default "RTS_World"))
  (bind _playercontroller (CallFunction|GetInstigatorPlayerController))
  (bind _returnvalue (Viewport|GetViewportSize))
  (bind _weapon (Variables|Default|GetWeapon))
  (bind _returnvalue_2 (Transformation|GetSocketTransform _weapon "Muzzle" TransformSpace))
  (bind _returnvalue_3 (/ _returnvalue 2.0))
  (bind (_x _y) (Math|Vector2D|BreakVector2D _returnvalue_3))
  (bind (_worldlocation _worlddirection) (Class|PlayerController|DeprojectScreenPositiontoWorld _playercontroller _x _y))
  (bind (_outhit _returnvalue_4) (Collision|LineTraceByChannel _worldlocation (+ _worldlocation (* _worlddirection 999999.0)) "TraceTypeQuery1" false 0 "ForOneFrame"))
  (return (.location _returnvalue_2) (Math|Vector|GetUnitDirection(Vector) (.location _returnvalue_2) (Math|Vector|SelectVector (.Location (Collision|BreakHitResult _outhit)) (.TraceEnd (Collision|BreakHitResult _outhit)) _returnvalue_4))))

(fn UseWeapon
  (bind (_ammoitem _found) (CallFunction|FindAmmo))
  (Utilities|IsValid (Variables|Default|GetAmmoItemRef)
    (:Is%20Valid
      _)
    (:Is%20Not%20Valid
      (if _found
        (Variables|Default|SetAmmoItemRef _ammoitem)
        (else
          (return false 0)))))
  (if (CallFunction|CanShoot)
    (CallFunction|UseAmmo)
    (bind (_used _weapon) (|CallParentFunction))
    (return _used _weapon)
    (else
      (return false 0))))

(fn UseAmmo
  (Default|RemoveItem (.Storage (CallFunction|IsinStorage)) (Variables|Default|GetAmmoItemRef) (== (Variables|/Game/KT_Storage/Storage/Items/BP_StorageItem.BP_StorageItem_C|GetQuantity (Variables|Default|GetAmmoItemRef)) 1))
  (Utilities|IsValid (Variables|Default|GetAmmoItemRef)
    (:Is%20Not%20Valid
      (Variables|Default|SetAmmoItemRef 0))))

(fn FindAmmo
  (bind _storage (CallFunction|IsinStorage))
  (bind _ammoitem (Variables|Default|GetAmmoItem))
  (bind (_item _wasfound) (Default|FindIteminStoragebyClass _storage _ammoitem))
  (if _wasfound
    (bind _asbp_ammo (Utilities|Casting|CastToBP_Ammo _item)
      (:then
        (return _asbp_ammo true))
      (:CastFailed
        (return 0 false)))
    (else
      (return 0 false))))

(fn CanShoot
  (return true))