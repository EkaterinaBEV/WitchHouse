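; BP_Weapon is a weapon item in the storage system, extending a parent item with equip, use and damage behavior.
; Equip and unequip call the parent logic, then switch the weapon component's collision off and back on.
; UseItem runs the parent, then UseWeapon, which prints a debug message and calls WeaponUsed.
; DealDamage applies damage to a valid hit actor with the instigator's controller, but nothing here calls it.
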(event EventBeginPlay
  (|CallParentFunction) ; This node is disabled and will not be called.\nDrag off pins to build functionality.
)

(event Collision|EventActorBeginOverlap
  (params (OtherActor :type Actor%20Object%20Reference))
  (|CallParentFunction OtherActor) ; This node is disabled and will not be called.\nDrag off pins to build functionality.
)

(event EventTick
  (params (DeltaSeconds :type Float%20%28single-precision%29))
  (|CallParentFunction DeltaSeconds) ; This node is disabled and will not be called.\nDrag off pins to build functionality.
)

(fn ConstructionScript
  (|CallParentFunction))

(fn DealDamage
  (params (Damage :type Float%20%28single-precision%29) (Hit :type Hit%20Result%20Structure) (DamageCauser :type Actor%20Object%20Reference))
  (bind _hitactor (Collision|BreakHitResult Hit))
  (Utilities|IsValid _hitactor
    (:Is%20Valid
      (Game|Damage|ApplyDamage _hitactor Damage (Game|GetInstigatorController) DamageCauser)
      (return true))
    (:Is%20Not%20Valid
      (return false))))

(fn UseWeapon
  (Development|PrintString "Weapon used!" true true "(R=1.000000,G=0.612458,B=0.000000,A=1.000000)")
  (Default|CallWeaponUsed self)
  (return true self))

(fn UseItem
  (|CallParentFunction)
  (bind _used (CallFunction|UseWeapon))
  (return _used))

(fn EquipItem
  (params (EquipToCharacter :type BP%20Character%20Object%20Reference))
  (bind _equipped (|CallParentFunction EquipToCharacter))
  (Collision|SetCollisionEnabled (Variables|Default|GetWeapon) "NoCollision")
  (return _equipped))

(fn UnequipItem
  (bind _equipped (|CallParentFunction))
  (Collision|SetCollisionEnabled (Variables|Default|GetWeapon) "QueryAndPhysics")
  (return _equipped))