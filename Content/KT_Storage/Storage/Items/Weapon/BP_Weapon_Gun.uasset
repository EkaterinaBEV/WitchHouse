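; BP_Weapon_Gun is a gun weapon Blueprint that fires a projectile when used, building on its parent's equip and use logic.
; Equipping disables collision on the Weapon component, and unequipping restores query and physics collision.
; UseWeapon calls ProjectileShot only when the parent's UseWeapon reports success, then returns whether the gun was used.
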(event EventBeginPlay
  (|CallParentFunction) ; This node is disabled and will not be called.\nDrag off pins to build functionality.
)

(event Collision|EventActorBeginOverlap
  (params (OtherActor :type Actor%20Object%20Reference))
  (|CallParentFunction OtherActor) ; This node is disabled and will not be called.\nDrag off pins to build functionality.
)

(event EventTick
  (params (DeltaSeconds :type Float%20%28single-precision%29))
  (|CallParentFunction DeltaSeconds) ; This node is disabled and will not be called.\nDrag off pins to build functionality.
)

(fn ConstructionScript
  (|CallParentFunction))

(fn EquipItem
  (params (EquipToCharacter :type BP%20Character%20Object%20Reference))
  (bind _equipped (|CallParentFunction EquipToCharacter))
  (Collision|SetCollisionEnabled (Variables|Default|GetWeapon) "NoCollision")
  (return _equipped))

(fn UnequipItem
  (bind _equipped (|CallParentFunction))
  (Collision|SetCollisionEnabled (Variables|Default|GetWeapon) "QueryAndPhysics")
  (return _equipped))

(fn UseWeapon
  (bind (_used _weapon) (|CallParentFunction))
  (if _used
    (CallFunction|ProjectileShot)
    (return true _weapon)
    (else
      (return false 0))))