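; Base storable item actor that characters pick up into a storage component through Interact.
; On storing, it records its storage and slot, sets owner and pawn instigator, hides and teleports to a far-off location.
; Simulating components found at construction are frozen and snapped to the root, then re-enabled when dropped to the world.
; A fly-away fix switches a character standing on the stored item to Falling.
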(fn ConstructionScript
  (Variables|Default|SetSceneComponents (Actor|GetComponentsByClass "/Script/Engine.SceneComponent"))
  (CallFunction|ScanforPhyzComponents))

(fn UseItem
  (return true))

(fn ItemAddedtoStorage
  (params (Storage :type BP%20Storage%20Component%20Object%20Reference) (Y :type Integer))
  (Variables|Components|SetOwningStorage Storage) ; Set показывает, что объект хранится именно в этом массиве
  (Variables|ItemInfo|SetInStorage true)
  (CallFunction|RelocateItem Y)
  (|Flyawayfix)
  (CallFunction|FreezePhyzComponents true)
  (Transformation|SetActorLocation "9999.000000,9999.000000,9999.000000" false true)
  (Rendering|SetActorHiddenInGame true)
  (Utilities|FlowControl|Sequence
    (:then_0
      ;[1 1 1] Set instigator (for weapon)
      (bind _aspawn (Utilities|Casting|CastToPawn (Components|GetOwner (Variables|Components|GetOwningStorage))))
      (Variables|Actor|SetInstigator _aspawn))
    (:then_1
      ;[1 1 1] Set owner
      (Actor|SetOwner (Components|GetOwner (Variables|Components|GetOwningStorage))))
    (:then_2
      (Default|CallItemAddedtoInventory self (Variables|Components|GetOwningStorage)))))

(fn ItemRemovedfromStorage
  (params (FromStorage :type BP%20Storage%20Component%20Object%20Reference))
  (Variables|Components|SetOwningStorage FromStorage)
  (Variables|ItemInfo|SetInStorage false)
  (Actor|SetOwner 0)
  (Variables|Actor|SetInstigator 0))

(fn DroppedtoWorld
  (params (Location :type Vector))
  (Transformation|SetActorLocation Location false true)
  (Rendering|SetActorHiddenInGame false)
  (CallFunction|FreezePhyzComponents false)
  (return true))

(fn IsinStorage
  ;[1 1 1] Находится в инвентаре и в каком именно
  (return (Variables|ItemInfo|GetInStorage) (Variables|Components|GetOwningStorage)))

(fn DestroyItem
  (Actor|DestroyActor))

(fn FreezePhyzComponents
  (params (Freeze :type Boolean))
  (for _array_element (Variables|Default|GetPhyzComponents)
    (Physics|SetSimulatePhysics _array_element (not Freeze))
    (if Freeze
      (Transformation|AttachComponentToComponent _array_element (Variables|Components|GetDefaultSceneRoot) "None" "SnapToTarget" "SnapToTarget" "KeepRelative" true))))

(fn GetInstigatorPlayerController
  (bind _asplayer_controller (Utilities|Casting|CastToPlayerController (Game|GetInstigatorController))
    (:then
      (return _asplayer_controller))
    (:CastFailed
      (return 0))))

(fn RemoveItem
  (bind (_instorage _storage) (CallFunction|IsinStorage))
  (if _instorage
    (Default|RemoveItem _storage self false)
    (else
      (CallFunction|DestroyItem))))

(fn LocateItem
  (return (Variables|InventoryInfo|GetPosY)))

(fn RelocateItem
  (params (Y :type Integer))
  (Variables|InventoryInfo|SetPosY Y)
  (Default|CallItemMoved self (Variables|InventoryInfo|GetPosY)))

(fn CheckifItemIsinSlot
  (params (Y :type Integer))
  (LocalVariables|SetL_Y Y)
  (if (== (LocalVariables|GetL_Y) (Variables|InventoryInfo|GetPosY))
    (return true)
    (else
      (return false))))

(fn Crafted)

(fn DropItem
  (Default|DropItemtoWorld (Variables|Components|GetOwningStorage) self))

(fn ScanforPhyzComponents
  (bind _output_get (LocalVariables|Setl_Components (Actor|GetComponentsByClass "/Script/Engine.SceneComponent")))
  (for _array_element _output_get
    (bind _asprimitive_component (Utilities|Casting|CastToPrimitiveComponent _array_element))
    (if (Physics|IsSimulatingPhysics _asprimitive_component "None")
      (Utilities|Array|Add (Variables|Default|GetPhyzComponents) _asprimitive_component))))

(fn Interact
  (params (Character :type BP%20Character%20Object%20Reference))
  (bind _added (Default|AddItem (Variables|/Game/KT_Character/Blueprints/BP_Character.BP_Character_C|GetBP_Comp_Storage Character) self))
  (return true (Utilities|String|SelectString "Item added" "No place, you greedy Goblin!" _added)))