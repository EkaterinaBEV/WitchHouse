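; BP_Harvestable_Bush is a harvestable bush whose berries become available again some time after being picked.
; On BeginPlay it binds BerriesHarvested to the items-harvested event, which starts a timer of BerriesSpawnTime and prints each harvested item's name.
; When the timer fires, SpawnBerries only clears the Harvested flag, with no actor or item spawning in this graph.
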(event Custom|BerriesHarvested
  (params (StorageComponent :type BP%20Storage%20Component%20Object%20Reference) (Items :type Array%20of%20BP%20Storage%20Item%20Object%20References))
  ;[1 1 1] Таймер, через время спаунится новая ягода
  (Utilities|Time|SetTimerbyFunctionName 0 "SpawnBerries" (Variables|Default|GetBerriesSpawnTime))
  (for _array_element Items
    (Development|PrintString (Utilities|GetDisplayName _array_element))))

(event EventBeginPlay
  (EventDispatchers|BindEventtoItemsHarvested (delegate Custom|BerriesHarvested)))

(event Collision|EventActorBeginOverlap
  (params (OtherActor :type Actor%20Object%20Reference))
  (|CallParentFunction OtherActor) ; This node is disabled and will not be called.\nDrag off pins to build functionality.
)

(event EventTick
  (params (DeltaSeconds :type Float%20%28single-precision%29))
  (|CallParentFunction DeltaSeconds) ; This node is disabled and will not be called.\nDrag off pins to build functionality.
)

(fn ConstructionScript
  (|CallParentFunction))

(fn SpawnBerries
  (Variables|Default|SetHarvested false))