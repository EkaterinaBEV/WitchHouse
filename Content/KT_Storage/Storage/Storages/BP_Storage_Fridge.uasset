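; Fridge storage actor that holds items in a storage component and can be interacted with by a character.
; Interact moves the fridge's first item into the character's storage; the reverse branch, adding the character's first item, is unreachable behind a hardcoded true condition.
; Tick prints every stored item's name as debug output, and a note marks the interaction logic as undecided.
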(event EventBeginPlay
  (|CallParentFunction) ; This node is disabled and will not be called.\nDrag off pins to build functionality.
)

(event Collision|EventActorBeginOverlap
  (params (OtherActor :type Actor%20Object%20Reference))
  (|CallParentFunction OtherActor) ; This node is disabled and will not be called.\nDrag off pins to build functionality.
)

(event EventTick
  (params (DeltaSeconds :type Float%20%28single-precision%29))
  (for _array_element (Default|GetItems (Variables|Default|GetBP_StorageComponent))
    (Development|PrintString (Variables|/Game/KT_Storage/Storage/Items/BP_StorageItem.BP_StorageItem_C|GetName _array_element) true true "(R=0.265093,G=1.000000,B=0.097409,A=1.000000)" 0.0))
  (Development|PrintString "Fridge Items: " true true "(R=0.099663,G=1.000000,B=0.000000,A=1.000000)" 0.0))

(fn ConstructionScript
  (|CallParentFunction))

(fn Interact
  (params (Character :type BP%20Character%20Object%20Reference))
  (bind _bp_storagecomponent (Variables|Default|GetBP_StorageComponent))
  ;[1 1 1] Подумать, что именно мне тут нужно
  (if true
    (bind _placed (Default|TransfertoAnotherStorage _bp_storagecomponent (Utilities|Array|Get(acopy) (Default|GetItems _bp_storagecomponent)) (Variables|/Game/KT_Character/Blueprints/BP_Character.BP_Character_C|GetBP_Comp_Storage Character)))
    (return _placed "Transfered")
    (else
      (bind _added (Default|AddItem (Variables|Default|GetBP_StorageComponent) (Utilities|Array|Get(acopy) (Default|GetItems (Variables|/Game/KT_Character/Blueprints/BP_Character.BP_Character_C|GetBP_Comp_Storage Character)))))
      (return _added "Transfered"))))