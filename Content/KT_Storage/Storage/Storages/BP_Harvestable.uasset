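; BP_Harvestable is an interactable world actor that gives items to a character's storage once, apparently berries given its failure message.
; Interact checks the Harvested flag and either calls Harvest on the character's BPCompStorage or returns failure with a message.
; Harvest creates the ItemsToHarvest through the storage component, broadcasts ItemsHarvested with the created items, then marks itself harvested.
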(event EventBeginPlay)

(event Collision|EventActorBeginOverlap
  (params (OtherActor :type Actor%20Object%20Reference)))

(event EventTick
  (params (DeltaSeconds :type Float%20%28single-precision%29)))

(fn ConstructionScript)

(fn Harvest
  (params (StorageComponent :type BP%20Storage%20Component%20Object%20Reference))
  (bind _createditems (Default|CreateItems StorageComponent (Variables|Default|GetItemsToHarvest)))
  (Default|CallItemsHarvested StorageComponent _createditems)
  (Variables|Default|SetHarvested true))

(fn Interact
  (params (Character :type BP%20Character%20Object%20Reference))
  (if (not (Variables|Default|GetHarvested))
    (CallFunction|Harvest (Variables|/Game/KT_Character/Blueprints/BP_Character.BP_Character_C|GetBP_Comp_Storage Character))
    (return true "Harvested")
    (else
      (return false "No berries"))))