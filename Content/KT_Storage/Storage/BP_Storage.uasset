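; BP_Storage is an interactable storage box that swaps items with the interacting character's storage component.
; Interact moves the box's first item to the character if that item is valid, otherwise it moves the character's first item into the box.
; It returns the transfer result with an empty message.
; Tick prints the box's item names to the screen every frame as debug output.
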(event EventBeginPlay)

(event Collision|EventActorBeginOverlap
  (params (OtherActor :type Actor%20Object%20Reference)))

(event EventTick
  (params (DeltaSeconds :type Float%20%28single-precision%29))
  (for _array_element (Default|GetItems (Variables|Default|GetBP_StorageComponent))
    (Development|PrintString (Variables|/Game/KT_Storage/Storage/Items/BP_StorageItem.BP_StorageItem_C|GetName _array_element) true true "(R=0.265093,G=1.000000,B=0.097409,A=1.000000)" 0.0))
  (Development|PrintString "Box Items: " true true "(R=0.099663,G=1.000000,B=0.000000,A=1.000000)" 0.0))

(fn ConstructionScript)

(fn Interact
  (params (Character :type BP%20Character%20Object%20Reference))
  (bind _bp_comp_storage (Variables|/Game/KT_Character/Blueprints/BP_Character.BP_Character_C|GetBP_Comp_Storage Character))
  (bind _bp_storagecomponent (Variables|Default|GetBP_StorageComponent))
  (bind _items (Default|GetItems _bp_storagecomponent))
  (bind _output (Utilities|Array|Get(acopy) _items))
  (Utilities|IsValid _output
    (:Is%20Valid
      (bind _placed (Default|TransfertoAnotherStorage (Variables|Default|GetBP_StorageComponent) _output _bp_comp_storage))
      (return _placed ""))
    (:Is%20Not%20Valid
      (bind _placed_2 (Default|TransfertoAnotherStorage _bp_comp_storage (Utilities|Array|Get(acopy) (Default|GetItems _bp_comp_storage)) (Variables|Default|GetBP_StorageComponent)))
      (return _placed_2 ""))))