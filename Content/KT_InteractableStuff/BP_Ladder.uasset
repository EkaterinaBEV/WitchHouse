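; BP_Ladder is a climbable ladder actor that puts a BP_Character into climbing while inside its Box trigger.
; Overlap sets the Climbing flag, switches movement to Flying and opens a Tick gate that snaps the character to face opposite the ladder's forward vector.
; Leaving the box, or the character hitting another actor, restores Walking and closes the gate.
; The author marks the per-tick rotation as a crude approach that needs animation.
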(event OnComponentBeginOverlap(Box)
  (params (OverlappedComponent :type Primitive%20Component%20Object%20Reference) (OtherActor :type Actor%20Object%20Reference) (OtherComp :type Primitive%20Component%20Object%20Reference) (OtherBodyIndex :type Integer) (bFromSweep :type Boolean) (SweepResult :type Hit%20Result%20Structure%20%28by%20ref%29))
  ;[1 1 1] Кривой способ, нужна анимация
  (bind _asbp_character (Utilities|Casting|CastToBP_Character OtherActor))
  (Collision|AssignOnActorHit _asbp_character (delegate Custom|OnActorHit_Event_0))
  (Variables|/Game/KT_Character/Blueprints/BP_Character.BP_Character_C|SetClimbing _asbp_character true)
  (Pawn|Components|CharacterMovement|SetMovementMode (Variables|/Script/Engine.Character|GetCharacterMovement _asbp_character) "MOVE_Flying" 0)
  (Utilities|FlowControl|Gate true) ; enters at Open
)

(event OnComponentEndOverlap(Box)
  (params (OverlappedComponent :type Primitive%20Component%20Object%20Reference) (OtherActor :type Actor%20Object%20Reference) (OtherComp :type Primitive%20Component%20Object%20Reference) (OtherBodyIndex :type Integer))
  ;[1 1 1] Кривой способ, нужна анимация
  (bind _asbp_character (Utilities|Casting|CastToBP_Character OtherActor))
  (Variables|/Game/KT_Character/Blueprints/BP_Character.BP_Character_C|SetClimbing _asbp_character false)
  (Pawn|Components|CharacterMovement|SetMovementMode (Variables|/Script/Engine.Character|GetCharacterMovement _asbp_character) "MOVE_Walking" 0)
  (Utilities|FlowControl|Gate true) ; enters at Close
)

(event Custom|OnActorHit_Event_0
  (params (SelfActor :type Actor%20Object%20Reference) (OtherActor :type Actor%20Object%20Reference) (NormalImpulse :type Vector) (Hit :type Hit%20Result%20Structure%20%28by%20ref%29))
  ;[1 1 1] Кривой способ, нужна анимация
  (if (!= OtherActor self)
    (Variables|/Game/KT_Character/Blueprints/BP_Character.BP_Character_C|SetClimbing (stale OnComponentEndOverlap(Box) _asbp_character) false)
    (Pawn|Components|CharacterMovement|SetMovementMode (Variables|/Script/Engine.Character|GetCharacterMovement (stale OnComponentEndOverlap(Box) _asbp_character)) "MOVE_Walking" 0)
    (Utilities|FlowControl|Gate true) ; enters at Close
  ))

(event EventBeginPlay)

(event Collision|EventActorBeginOverlap
  (params (OtherActor :type Actor%20Object%20Reference)))

(event EventTick
  (params (DeltaSeconds :type Float%20%28single-precision%29))
  ;[1 1 1] Кривой способ, нужна анимация
  (Utilities|FlowControl|Gate true
    (:Exit
      (Transformation|SetActorRotation (stale OnComponentBeginOverlap(Box) _asbp_character) (Math|Conversions|RotationFromXVector (* (Transformation|GetActorForwardVector) -1)) true))))

(fn ConstructionScript)