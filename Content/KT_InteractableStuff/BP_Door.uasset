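; BP_Door is an interactable door that opens for a character holding a key and closes automatically.
; Interact checks one equipment slot for a BP_Key, then plays the OpenTheDoor timeline, which drives Scene1's rotation.
; Leaving the Box starts a Tick-based countdown that reverses the timeline through CloseDoor.
; Re-entering only clears the leftover StopTimer handle, so the countdown keeps running.
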(event OnComponentBeginOverlap(Box)
  (params (OverlappedComponent :type Primitive%20Component%20Object%20Reference) (OtherActor :type Actor%20Object%20Reference) (OtherComp :type Primitive%20Component%20Object%20Reference) (OtherBodyIndex :type Integer) (bFromSweep :type Boolean) (SweepResult :type Hit%20Result%20Structure%20%28by%20ref%29))
  ;[1 1 1] Нужна другая логика
  (Utilities|Time|ClearandInvalidateTimerbyHandle (Variables|Default|GetStopTimer)))

(event OnComponentEndOverlap(Box)
  (params (OverlappedComponent :type Primitive%20Component%20Object%20Reference) (OtherActor :type Actor%20Object%20Reference) (OtherComp :type Primitive%20Component%20Object%20Reference) (OtherBodyIndex :type Integer))
  ;[1 1 1] Нужна другая логика
  (Variables|Default|SetTimer 3.0))

(event EventTick
  (params (DeltaSeconds :type Float%20%28single-precision%29))
  ;[1 1 1] Нужна другая логика
  (if (> (Variables|Default|GetTimer) 0.0)
    (bind _output_get (Variables|Default|SetTimer (- (Variables|Default|GetTimer) DeltaSeconds)))
    (if (<= _output_get 0.0)
      (CallFunction|CloseDoor))))

(event Collision|EventActorBeginOverlap
  (params (OtherActor :type Actor%20Object%20Reference)))

(event EventBeginPlay)

(fn ConstructionScript)

(fn KeyinHand
  (return (Variables|Default|GetHandOccupied) (Variables|Default|GetHand) (Variables|Default|GetKey)))

(fn CloseDoor
  (Components|Timeline|ReversefromEnd (Variables|Default|GetOpenTheDoor)))

(fn Interact
  (params (Character :type BP%20Character%20Object%20Reference))
  (bind _bp_comp_equipment (Variables|/Game/KT_Character/Blueprints/BP_Character.BP_Character_C|GetBP_Comp_Equipment Character))
  (bind (_equipped _item) (Default|PartEquipped _bp_comp_equipment "NewEnumerator0"))
  (if _equipped
    (Utilities|Casting|CastToBP_Key _item
      (:then
        (Audio|Components|Audio|Play (Variables|Default|GetOpenTheDoor))
        (return true "Door is open"))
      (:CastFailed
        (return false "You need key")))
    (else
      (Development|PrintString "You need key"))))